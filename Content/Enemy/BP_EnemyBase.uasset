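; Base enemy character Blueprint providing sword combat actions, a patrol route getter and movement speed control.
; Attack, wield and sheathe events play montages, then call event dispatchers on completion; only Attack also does so when interrupted.
; Montage notifies time the sword's spawn and socket attachment to the hand, and its destruction, updating the wielding flag.
; SetMovementSpeed maps idle-to-sprint states to walk speed.
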(event Custom|Attack
  ;[1 1 1] Attack Animation
  (Animation|Montage|PlayMontage (Variables|Character|GetMesh) "/Game/Enemy/Animations/Montage_Sword_Slash.Montage_Sword_Slash"
    (:OnCompleted
      _)
    (:OnInterrupted
      _))
  (Default|CallOnAttackEnd))

(event Custom|WieldSword
  ;[1 1 1] Wield Sword
  (bind _notifyname (Animation|Montage|PlayMontage (Variables|Character|GetMesh) "/Game/Enemy/Animations/AnimM_UnsheatheSword.AnimM_UnsheatheSword")
    (:OnCompleted
      (Default|CallOnWieldSword))
    (:OnNotifyBegin
      (switch name _notifyname
        (:UnsheatheSword
          (bind _returnvalue (Game|SpawnActorfromClass "/Game/Weapons/BP_Sword.BP_Sword_C" (Transformation|GetActorTransform) "Undefined" "MultiplyWithRoot" 0 0))
          (bind _output_get (Variables|Default|SetSwordActor _returnvalue))
          (Transformation|AttachComponentToComponent _output_get (Variables|Character|GetMesh) "hand_r_sword_socket" "SnapToTarget" "SnapToTarget" "SnapToTarget" true)
          (Variables|Default|SetIsWieldingWeapon true))))))

(event Custom|SheatheSword
  (bind _notifyname (Animation|Montage|PlayMontage (Variables|Character|GetMesh) "/Game/Enemy/Animations/AnimM_SheatheSword.AnimM_SheatheSword")
    (:OnCompleted
      (Default|CallOnSheatheSword))
    (:OnNotifyBegin
      (switch name _notifyname
        (:SheatheSword
          (Actor|DestroyActor (Variables|Default|GetSwordActor))
          (Variables|Default|SetIsWieldingWeapon false))))))

(event EventBeginPlay)

(fn ConstructionScript)

(fn GetPatrolRoute
  (return (Variables|AI|GetPatrolRoute)))

(fn SetMovementSpeed
  (params (Speed :type E_MovementSpeed%20Enum :default "NewEnumerator0"))
  (bind _output_get (Variables|/Script/Engine.CharacterMovementComponent|SetMaxWalkSpeed (Variables|Character|GetCharacterMovement) (Utilities|Select :Index Speed :NewEnumerator0 0.0 :NewEnumerator1 1e+02 :NewEnumerator2 3e+02 :NewEnumerator3 5e+02)))
  (return _output_get))