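; Enemy pool that pre-spawns BP_EnemyBase AI pawns for its owner, with reuse not yet implemented.
; On BeginPlay it loops on AmountOfEnemies, spawning each pawn with BT_EnemyBase at the owner's transform and attaching it to the owner.
; Each pass binds ReturnToPool to OnEnemyKilled through GetActorOfClass, so it targets the first enemy found rather than the new spawn.
; ReturnToPool is an empty stub.
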(event Custom|ReturnToPool)

(event EventBeginPlay
  (bind _returnvalue (Components|GetOwner))
  (for _index (range 0 (Variables|Default|GetAmountOfEnemies))
    (bind _returnvalue_2 (AI|SpawnAIFromClass "/Game/Enemy/BP_EnemyBase.BP_EnemyBase_C" "/Game/Enemy/AI/BT_EnemyBase.BT_EnemyBase" (Transformation|GetActorLocation _returnvalue) (Transformation|GetActorRotation _returnvalue) false 0))
    (Transformation|AttachActorToActor _returnvalue_2 (Components|GetOwner) "None" "KeepWorld" "KeepWorld" "KeepWorld" true)
    (bind _returnvalue_3 (Actor|GetActorOfClass "/Game/Enemy/BP_EnemyBase.BP_EnemyBase_C"))
    (EventDispatchers|AssignOnEnemyKilled _returnvalue_3 (delegate Custom|ReturnToPool))))