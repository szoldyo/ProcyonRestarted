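; BP_ProcyonGamemode is a game mode Blueprint that sets the game's quality levels on BeginPlay, in a block labeled Potato Mode.
; A Sequence pushes one GameQuality value into the Game User Settings scalability groups, covering rendering categories such as textures, shadows and foliage, plus audio quality.
; Each branch calls ApplySettings separately, and shading quality is set twice.
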(event EventBeginPlay
  ;[1 1 1] Potato Mode
  (Utilities|FlowControl|Sequence
    (:then_0
      (bind _returnvalue (Settings|GetGameUserSettings))
      (Class|GameUserSettings|SetTextureQuality _returnvalue (Variables|Default|GetGame%20Quality))
      (Class|GameUserSettings|ApplySettings _returnvalue true))
    (:then_1
      (bind _returnvalue_2 (Settings|GetGameUserSettings))
      (Class|GameUserSettings|SetPostProcessingQuality _returnvalue_2 (Variables|Default|GetGame%20Quality))
      (Class|GameUserSettings|ApplySettings _returnvalue_2 true))
    (:then_2
      (bind _returnvalue_3 (Settings|GetGameUserSettings))
      (Class|GameUserSettings|SetAntiAliasingQuality _returnvalue_3 (Variables|Default|GetGame%20Quality))
      (Class|GameUserSettings|ApplySettings _returnvalue_3 true))
    (:then_3
      (bind _returnvalue_4 (Settings|GetGameUserSettings))
      (Class|GameUserSettings|SetShadowQuality _returnvalue_4 (Variables|Default|GetGame%20Quality))
      (Class|GameUserSettings|ApplySettings _returnvalue_4 true))
    (:then_4
      (bind _returnvalue_5 (Settings|GetGameUserSettings))
      (Class|GameUserSettings|SetShadingQuality _returnvalue_5 (Variables|Default|GetGame%20Quality))
      (Class|GameUserSettings|ApplySettings _returnvalue_5 true))
    (:then_5
      (bind _returnvalue_6 (Settings|GetGameUserSettings))
      (Class|GameUserSettings|SetViewDistanceQuality _returnvalue_6 (Variables|Default|GetGame%20Quality))
      (Class|GameUserSettings|ApplySettings _returnvalue_6 true))
    (:then_6
      (bind _returnvalue_7 (Settings|GetGameUserSettings))
      (Class|GameUserSettings|SetReflectionQuality _returnvalue_7 (Variables|Default|GetGame%20Quality))
      (Class|GameUserSettings|ApplySettings _returnvalue_7 true))
    (:then_7
      (bind _returnvalue_8 (Settings|GetGameUserSettings))
      (Class|GameUserSettings|SetVisualEffectQuality _returnvalue_8 (Variables|Default|GetGame%20Quality))
      (Class|GameUserSettings|ApplySettings _returnvalue_8 true))
    (:then_8
      (bind _returnvalue_9 (Settings|GetGameUserSettings))
      (Class|GameUserSettings|SetFoliageQuality _returnvalue_9 (Variables|Default|GetGame%20Quality))
      (Class|GameUserSettings|ApplySettings _returnvalue_9 true))
    (:then_9
      (bind _returnvalue_10 (Settings|GetGameUserSettings))
      (Class|GameUserSettings|SetShadingQuality _returnvalue_10 (Variables|Default|GetGame%20Quality))
      (Class|GameUserSettings|ApplySettings _returnvalue_10 true))
    (:then_10
      (bind _returnvalue_11 (Settings|GetGameUserSettings))
      (Class|GameUserSettings|SetAudioQualityLevel _returnvalue_11 (Variables|Default|GetGame%20Quality))
      (Class|GameUserSettings|ApplySettings _returnvalue_11 true))))

(fn ConstructionScript)